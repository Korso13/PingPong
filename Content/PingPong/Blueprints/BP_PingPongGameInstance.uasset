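; Game instance for the PingPong game that handles hosting, finding and joining online sessions.
; CreateNewSession creates a session, then opens the given map with the server option on success.
; GetServers searches for a few sessions, prints their details and passes non-empty results to the W_Client_MainMenu widget.
; JoinSession joins a chosen result, and failures in all three events are only reported with debug prints.
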(event Custom|Create%20New%20Session
  (params (MaxPlayers :type Integer) (bLAN :type Boolean) (MapName :type Name :default "Level1"))
  ;[0.4655 0.4928 1] Function creating new listenning server session
  (|Session (Game|GetPlayerController 0) MaxPlayers bLAN
    (:OnSuccess
      (Game|OpenLevel(byName) MapName true "-server")
      (Development|PrintString "GameInstance: Game Level created! ---------------------------"))
    (:OnFailure
      (Development|PrintString "Session creation failed!!!" true true "(R=1.000000,G=0.018600,B=0.000000,A=1.000000)"))))

(event Custom|GetServers
  (params (bSearchLAN :type Boolean) (MainMenuRef :type User%20Widget%20Object%20Reference))
  ;[0.3186 1 0.3008] Find sessions
  (bind _results (|FindSessions (Game|GetPlayerController 0) 5 bSearchLAN)
    (:OnSuccess
      (for _array_element _results
        (Development|PrintString (Utilities|String|Append "Server name: " (Class|FindSessionsCallbackProxy|GetServerName _array_element) " Players: " (Utilities|String|ToString(Integer) (Class|FindSessionsCallbackProxy|GetCurrentPlayers _array_element)) "/" (Utilities|String|ToString(Integer) (Class|FindSessionsCallbackProxy|GetMaxPlayers _array_element)) " Ping: " (Utilities|String|ToString(Integer) (Class|FindSessionsCallbackProxy|GetPinginMs _array_element)))))
      ;;[0.4161 0.2142 1] Return server search results to widget
      (bind _output_get (Variables|Default|SetFoundServersArray _results))
      ;;;[1 0 0.09242] Check if any servers were found
      (if (> (Utilities|Array|Length _output_get) 0)
        (bind _asw_client_main_menu (Utilities|Casting|CastToW_Client_MainMenu MainMenuRef))
        (Default|GetServerSearchResults _asw_client_main_menu _output_get)))
    (:OnFailure
      (Development|PrintString "No servers found!" true true "(R=1.000000,G=0.008761,B=0.000000,A=1.000000)"))))

(event Custom|JoinSession
  (params (Server :type Blueprint%20Session%20Result%20Structure))
  ;[1 0.3541 0.364] Join session
  (|JoinSession (Game|GetPlayerController 0) Server
    (:OnFailure
      (Development|PrintString "Couldn't join the game!"))))